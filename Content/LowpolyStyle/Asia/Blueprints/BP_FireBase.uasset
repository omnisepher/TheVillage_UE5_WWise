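; BP_FireBase is a fire actor with particle effects and Wwise audio that burns the wizard character on contact.
; BeginPlay posts the fire's sound event, and Tick runs HealthManagement, which stops both particle effects and audio whenever IsBurning is false.
; While burning, a gate toggled by FireCollision overlap begin and end drains the overlapping WizardCH_BP's Health at a fixed rate scaled by delta time.
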(event `self.ReceiveBeginPlay`
  (`AkGameObject.PostAssociatedAkEventAsync` :`self` (`self.FireBase`)))

(event `self.ReceiveTick`
  (params (DeltaSeconds :type "Float (single-precision)"))
  (bind _isburning (`self.IsBurning`))
  (`|ExecutionSequence`
    (:`then_0`
      (`|ExecutionSequence`
        (:`then_0`
          (if (not _isburning)
            (`ActorComponent.Deactivate` (`self.PS_Fire`))
            (`AkGameObject.Stop` (`self.FireBase`))
            (`ActorComponent.Deactivate` (`self.PS_BluePlume`))))
        (:`then_1`
          (if _isburning
            (bind _aswizard_ch_bp (cast `/Game/BattleWizardPolyart/CharacterBP/WizardCH_BP` (stale `self.FireCollision.OnComponentBeginOverlap` OtherActor)))
            (`/Engine/EditorBlueprintResources/StandardMacros.Gate` true :!label _label
              (:`Exit`
                (set `WizardChar.Health` (- (`WizardChar.Health` _aswizard_ch_bp) (* DeltaSeconds 10.0)) _aswizard_ch_bp)))))))))

(event `self.FireCollision.OnComponentBeginOverlap`
  (params (OverlappedComponent :type "PrimitiveComponent Object Reference") (OtherActor :type "Actor Object Reference") (OtherComp :type "PrimitiveComponent Object Reference") (OtherBodyIndex :type Integer) (bFromSweep :type Boolean) (SweepResult :type "HitResult Structure (by ref)"))
  (goto _label :!via `Open`))

(event `self.FireCollision.OnComponentEndOverlap`
  (params (OverlappedComponent :type "PrimitiveComponent Object Reference") (OtherActor :type "Actor Object Reference") (OtherComp :type "PrimitiveComponent Object Reference") (OtherBodyIndex :type Integer))
  (goto _label :!via `Close`))

(fn `UserConstructionScript`
  (set `self.BlueFireFX` (`self.PS_BluePlume`)))